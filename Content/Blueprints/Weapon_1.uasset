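; Automatic hitscan weapon that fires toward the point under the first player's cursor.
; PullTrigger fires once through a DoOnce and starts a looping timer at the FireRate interval, which ReleaseTrigger clears and resets.
; Each shot plays a shrunken explosion at the muzzle, line-traces to the cursor hit, spawns an impact explosion and sends damage through the ICharacter interface.
; An unconnected LazerProjectile spawn-and-impulse branch never runs.
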(event `PullTrigger`
  (`/Engine/EditorBlueprintResources/StandardMacros.DoOnce` false :!label _label
    (:`Completed`
      (`self.Fire`)
      (bind _returnvalue (`KismetSystemLibrary.K2_SetTimerDelegate` (delegate `Fire`) (/ 1.0 (`self.FireRate`)) true))
      (set `self.FireTimer` _returnvalue))))

(event `ReleaseTrigger`
  (`KismetSystemLibrary.K2_ClearAndInvalidateTimerHandle` (`self.FireTimer`))
  (goto _label :!via `Reset`))

(event `Fire`
  (bind _mesh (`self.Mesh`))
  (bind _returnvalue (`GameplayStatics.SpawnEmitterAttached` "/Game/StarterContent/Particles/P_Explosion.P_Explosion" _mesh "Muzzle" (0.0 0.0 0.0) (struct) "SnapToTarget"))
  (`SceneComponent.K2_SetWorldTransform` _returnvalue (`KismetMathLibrary.MakeTransform` (.location (`SceneComponent.K2_GetComponentToWorld` _returnvalue)) (.rotation (`SceneComponent.K2_GetComponentToWorld` _returnvalue)) (/ (.scale (`SceneComponent.K2_GetComponentToWorld` _returnvalue)) 5.0)) false false)
  (bind (_outhit _returnvalue_2) (`KismetSystemLibrary.LineTraceSingleForObjects` (.location (`SceneComponent.GetSocketTransform` _mesh "Muzzle" "RTS_World")) (`.Location` (`GameplayStatics.BreakHitResult` (`PlayerController.GetHitResultUnderCursorForObjects` (`GameplayStatics.GetPlayerController` 0) (`|MakeArray` "ObjectTypeQuery1" "ObjectTypeQuery2" "ObjectTypeQuery3" "ObjectTypeQuery4" "ObjectTypeQuery6" :!type "EObjectTypeQuery Enum") true))) (`|MakeArray` "ObjectTypeQuery1" "ObjectTypeQuery2" "ObjectTypeQuery3" "ObjectTypeQuery4" "ObjectTypeQuery6" :!type "EObjectTypeQuery Enum") true))
  (if _returnvalue_2
    (bind (_bblockinghit _binitialoverlap _time _location _impactpoint _normal _impactnormal _physmat _hitactor) (`GameplayStatics.BreakHitResult` _outhit))
    (`GameplayStatics.SpawnEmitterAtLocation` "/Game/StarterContent/Particles/P_Explosion.P_Explosion" _location (`KismetMathLibrary.Conv_VectorToRotator` _normal))
    (if (`KismetSystemLibrary.DoesImplementInterface` _hitactor "/Game/Blueprints/iCharacter.iCharacter_C")
      (message `/Game/Blueprints/iCharacter.ReceiveDamage` _hitactor "NewEnumerator0" _outhit))))

(fn `UserConstructionScript`)