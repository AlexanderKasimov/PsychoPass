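; Building-tool floor Blueprint that fills a grid with mesh blocks, sized by X and Y splines.
; The construction script derives block counts at 200-unit spacing, resizes the editable block array to match, then calls BuildBlock per entry.
; Blocks take X and Z from one spline and Y from the other, unrotated, with per-block or master material.
; The master-mesh branch is unfinished: it adds a destructible component but sets the mesh on None.
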(event `self.ReceiveBeginPlay`)

(event `Unhide`
  (`self.SetActorHiddenInGame` false))

(fn `BuildBlock`
  (params (BlockInfo :type "/Game/Blueprints/BuildingTools/BuildingBlockInfo Structure") (Index :type Integer))
  (locals (LocalBlockInfo :type "/Game/Blueprints/BuildingTools/BuildingBlockInfo Structure") (LocalIndex :type Integer) (LocalMesh :type "StaticMeshComponent Object Reference"))
  (set `local.LocalBlockInfo` BlockInfo)
  (set `local.LocalIndex` Index)
  (`|ExecutionSequence`
    (:`then_0`
      (if (`self.UseMasterMesh`)
        (`AddComponent|NODE_AddDestructibleComponent-0`)
        (bind _output_get (set `local.LocalMesh` null))
        (`StaticMeshComponent.SetStaticMesh` _output_get (`self.MasterMesh`))
        (else
          (bind _returnvalue (`AddComponent|NODE_AddStaticMeshComponent-2` :`bManualAttachment` true :`RelativeTransform` (`KismetMathLibrary.MakeTransform` (`KismetMathLibrary.MakeVector` (.x (`SplineComponent.GetLocationAtDistanceAlongSpline` (`self.SplineXAxis`) (* (mod (`local.LocalIndex`) (`self.BlockCountX`)) 200.0) "World")) (.y (`SplineComponent.GetLocationAtDistanceAlongSpline` (`self.SplineYAxis`) (* (/ (`local.LocalIndex`) (`self.BlockCountX`)) 200.0) "World")) (.z (`SplineComponent.GetLocationAtDistanceAlongSpline` (`self.SplineXAxis`) (* (mod (`local.LocalIndex`) (`self.BlockCountX`)) 200.0) "World"))))))
          (bind _output_get_2 (set `local.LocalMesh` _returnvalue))
          (`StaticMeshComponent.SetStaticMesh` _output_get_2 (`.Mesh_2_F2E579724B4DF508E4A325ABFAE8C200` (break `/Game/Blueprints/BuildingTools/BuildingBlockInfo` (`local.LocalBlockInfo`)))))))
    (:`then_1`
      (if (`self.UseMasterMaterial`)
        (`PrimitiveComponent.SetMaterial` (`local.LocalMesh`) 0 (`self.MasterMatrialInst`))
        (else
          (`PrimitiveComponent.SetMaterial` (`local.LocalMesh`) 0 (`.Material_6_60A126144357AC6218A5DA80B334F1C2` (break `/Game/Blueprints/BuildingTools/BuildingBlockInfo` (`local.LocalBlockInfo`)))))))))

(fn `UserConstructionScript`
  (bind _buildingblockelements (`self.BuildingBlockElements`))
  (`|ExecutionSequence`
    (:`then_0`
      (set `self.BlockCountX` (`.ReturnValue` (`KismetMathLibrary.FMod` (`SplineComponent.GetSplineLength` (`self.SplineXAxis`)) 200.0))))
    (:`then_1`
      (set `self.BlockCountY` (`.ReturnValue` (`KismetMathLibrary.FMod` (`SplineComponent.GetSplineLength` (`self.SplineYAxis`)) 200.0))))
    (:`then_2`
      (`/Engine/EditorBlueprintResources/StandardMacros.CompareInt` (`KismetArrayLibrary.Array_Length` (`self.BuildingBlockElements`)) (* (`self.BlockCountX`) (`self.BlockCountY`)) :!label _label
        (:`>`
          (`KismetArrayLibrary.Array_Remove` _buildingblockelements (`KismetArrayLibrary.Array_LastIndex` _buildingblockelements))
          (goto _label))
        (:`<`
          (`KismetArrayLibrary.Array_Add` (`self.BuildingBlockElements`) (make `/Game/Blueprints/BuildingTools/BuildingBlockInfo` (`self.MasterMesh`) (`self.MasterMatrialInst`)))
          (goto _label))))
    (:`then_3`
      (for (_array_element _array_index) (`self.BuildingBlockElements`)
        (`self.BuildBlock` _array_element _array_index)))))