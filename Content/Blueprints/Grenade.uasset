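; Grenade actor that explodes on its first hit and dismembers enemies caught in the blast.
; On spawn it randomizes its dynamic material's color and keeps DamageSphere collision off.
; Impact spawns an explosion emitter and radial force component, enables DamageSphere, then sets force strength and destroys itself after staged delays.
; Overlapped EnemyCharacters ragdoll, lose capsule collision, get a limited lifespan and have every bone constraint broken.
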(event `self.ReceiveBeginPlay`
  ;[1 1 1] Disable DamageSphere and Set Random Material Color
  (`/Game/Blueprints/MaterialComponent.RandomizeVectorParameter` (`self.MaterialComponent`) (`self.GrenadeMat`) "Color")
  (`PrimitiveComponent.SetCollisionEnabled` (`self.DamageSphere`) "NoCollision"))

(event `self.Mesh.OnComponentHit`
  (params (HitComponent :type "PrimitiveComponent Object Reference") (OtherActor :type "Actor Object Reference") (OtherComp :type "PrimitiveComponent Object Reference") (NormalImpulse :type "Vector Structure") (Hit :type "HitResult Structure (by ref)"))
  (bind (_bblockinghit _binitialoverlap _time _location) (`GameplayStatics.BreakHitResult` Hit))
  ;[1 1 1] Explosion When Hit Something
  (`/Engine/EditorBlueprintResources/StandardMacros.DoOnce` false
    (:`Completed`
      (`GameplayStatics.SpawnEmitterAtLocation` "/Game/StarterContent/Particles/P_Explosion.P_Explosion" _location)
      (bind _returnvalue (`AddComponent|NODE_AddRadialForceComponent-0`))
      (`SceneComponent.K2_SetWorldLocation` _returnvalue _location false false)
      (`PrimitiveComponent.SetCollisionEnabled` (`self.DamageSphere`) "QueryAndPhysics")
      (`KismetSystemLibrary.Delay` 0.4)
      (set `RadialForceComponent.ForceStrength` 200000.0 _returnvalue)
      (`KismetSystemLibrary.Delay` 0.4)
      (`self.K2_DestroyActor`))))

(event `self.DamageSphere.OnComponentBeginOverlap`
  (params (OverlappedComponent :type "PrimitiveComponent Object Reference") (OtherActor :type "Actor Object Reference") (OtherComp :type "PrimitiveComponent Object Reference") (OtherBodyIndex :type Integer) (bFromSweep :type Boolean) (SweepResult :type "HitResult Structure (by ref)"))
  ;[1 1 1] Dismember All Enemies in DamageSphere
  (bind _asenemy_character (cast `/Game/Blueprints/EnemyCharacter` OtherActor))
  (`PrimitiveComponent.SetSimulatePhysics` (`Character.Mesh` _asenemy_character) true)
  (`PrimitiveComponent.SetCollisionEnabled` (`Character.CapsuleComponent` _asenemy_character) "NoCollision")
  (`self.SetLifeSpan` _asenemy_character 15.0)
  (for _index (range (`SkinnedMeshComponent.GetNumBones` (`Character.Mesh` _asenemy_character)))
    (bind _mesh (`Character.Mesh` _asenemy_character))
    (`SkeletalMeshComponent.BreakConstraint` _mesh (0.0 0.0 0.0) (0.0 0.0 0.0) (`SkinnedMeshComponent.GetBoneName` _mesh _index))))

(fn `UserConstructionScript`
  (bind _returnvalue (`PrimitiveComponent.CreateDynamicMaterialInstance` (`self.Mesh`) 0 null))
  (set `self.GrenadeMat` _returnvalue))