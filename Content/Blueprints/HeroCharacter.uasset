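; Player hero for a cursor-aimed shooter with world-axis movement, impulse-thrown grenades and a pause toggle.
; BeginPlay attaches the starting weapon to the mesh and shows a crosshair cursor; Tick turns character and weapon toward the cursor hit, while Fire drives the trigger.
; The first Damage event ragdolls the mesh, constraining its spine to the hit component until a random delay breaks it.
; Building-hiding and stick-aim logic is disconnected.
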(event `self.ReceiveBeginPlay`
  (bind _returnvalue (`GameplayStatics.GetPlayerController` 0))
  ;[1 1 1] Spawn Weapon and Attach It To Capsule, Then Show Mouse Cursor and Set It to Crosshair (On BeginPlay)
  (`|ExecutionSequence`
    (:`then_0`
      (bind _returnvalue_2 (`|SpawnActorFromClass` (`self.StartingWeapon`) (`SceneComponent.GetSocketTransform` (`self.Mesh`) "WeaponSocket" "RTS_World") "Undefined" "OverrideRootScale" null null))
      (bind _asweapon_1 (cast `/Game/Blueprints/Weapon_1` _returnvalue_2))
      (bind _output_get (set `self.CurWeapon` _asweapon_1))
      (`SceneComponent.K2_AttachToComponent` (`Actor.RootComponent` _output_get) (`self.Mesh`) "lowerarm_rSocket" "SnapToTarget" "SnapToTarget" "KeepRelative" true))
    (:`then_1`
      (set `PlayerController.bShowMouseCursor` true _returnvalue)
      (set `PlayerController.CurrentMouseCursor` "Crosshairs" _returnvalue))))

(event `self.ReceiveTick`
  (params (DeltaSeconds :type "Float (single-precision)"))
  ;[1 1 1] Rotating Character to Crosshair Then Hide/Unhide System (Will be Changed) Work (On EventTick)
  (`|ExecutionSequence`
    (:`then_0`
      (`self.RotateToCursor`))))

(event `InputAxis|MoveUp`
  (params (AxisValue :type "Float (single-precision)"))
  ;[1 1 1] Movement
  (`self.AddMovementInput` (1.0 0.0 0.0) AxisValue))

(event `InputAxis|MoveRight`
  (params (AxisValue :type "Float (single-precision)"))
  ;[1 1 1] Movement
  (`self.AddMovementInput` (0.0 1.0 0.0) AxisValue))

(event `InputAction|Grenade`
  (params (Key :type "Key Structure"))
  (bind _rotation (.rotation (`self.GetTransform`)))
  (bind _returnvalue (`KismetMathLibrary.GetForwardVector` _rotation))
  ;[1 1 1] Grenade Throwing
  (:`Pressed`
    (bind _returnvalue_2 (`|SpawnActorFromClass` "/Game/Blueprints/Grenade.Grenade_C" (`KismetMathLibrary.MakeTransform` (+ (.location (`self.GetTransform`)) (* _returnvalue 100.0)) _rotation) "Undefined" "OverrideRootScale" null null))
    (bind _output_get (set `self.CurGrenade` _returnvalue_2))
    (`PrimitiveComponent.SetSimulatePhysics` (`/Game/Blueprints/Grenade.Mesh` _output_get) true)
    (`PrimitiveComponent.AddImpulse` (`/Game/Blueprints/Grenade.Mesh` (`self.CurGrenade`)) (+ (* _returnvalue 700.0) (* (`KismetMathLibrary.GetUpVector` _rotation) 1000.0)) "None" false)))

(event `self.CameraTraceBox.OnComponentBeginOverlap`
  (params (OverlappedComponent :type "PrimitiveComponent Object Reference") (OtherActor :type "Actor Object Reference") (OtherComp :type "PrimitiveComponent Object Reference") (OtherBodyIndex :type Integer) (bFromSweep :type Boolean) (SweepResult :type "HitResult Structure (by ref)"))
  ;[1 0 0] Overlap Based Hide/Unhide (Rejected)
)

(event `self.CameraTraceBox.OnComponentEndOverlap`
  (params (OverlappedComponent :type "PrimitiveComponent Object Reference") (OtherActor :type "Actor Object Reference") (OtherComp :type "PrimitiveComponent Object Reference") (OtherBodyIndex :type Integer))
  ;[1 0 0] Overlap Based Hide/Unhide (Rejected)
)

(event `InputAction|Fire`
  (params (Key :type "Key Structure"))
  (bind _curweapon (`self.CurWeapon`))
  ;[1 1 1] Shooting System
  (:`Pressed`
    (`/Game/Blueprints/Weapon_1.PullTrigger` _curweapon))
  (:`Released`
    (`/Game/Blueprints/Weapon_1.ReleaseTrigger` _curweapon)))

(event `InputAxis|LookUp`
  (params (AxisValue :type "Float (single-precision)"))
  ;[1 0 0] Rotating/Firing System (Changed for New)
)

(event `InputAxis|LookRight`
  (params (AxisValue :type "Float (single-precision)"))
  ;[1 0 0] Rotating/Firing System (Changed for New)
)

(event `InputAction|Pause` :paused true
  (params (Key :type "Key Structure"))
  ;[1 1 1] Pause/Unpause Game
  (:`Pressed`
    (`/Engine/EditorBlueprintResources/StandardMacros.FlipFlop`
      (:`A`
        (`GameplayStatics.SetGamePaused` true))
      (:`B`
        (`GameplayStatics.SetGamePaused` false)))))

(event `/Game/Blueprints/iCharacter.ReceiveDamage`
  (params (DamageType :type "/Game/Blueprints/Enum_DamageType Enum" :default "NewEnumerator0") (HitInfo :type "HitResult Structure"))
  (bind (_bblockinghit _binitialoverlap _time _location _impactpoint _normal _impactnormal _physmat _hitactor _hitcomponent) (`GameplayStatics.BreakHitResult` HitInfo))
  (`/Engine/EditorBlueprintResources/StandardMacros.DoOnce` false
    (:`Completed`
      (`PrimitiveComponent.SetCollisionEnabled` (`self.CapsuleComponent`) "NoCollision")
      (`PrimitiveComponent.SetSimulatePhysics` (`self.Mesh`) true)
      (bind _returnvalue (`AddComponent|NODE_AddPhysicsConstraintComponent-0`))
      (`SceneComponent.K2_SetWorldLocation` _returnvalue _location false false)
      (`PhysicsConstraintComponent.SetConstrainedComponents` _returnvalue (`self.Mesh`) "spine_01" _hitcomponent "R_forearm")
      (`KismetSystemLibrary.Delay` (`KismetMathLibrary.RandomFloatInRange` 4.5 15.5))
      (`PhysicsConstraintComponent.BreakConstraint` _returnvalue))))

(fn `RotateToCursor`
  (bind _curweapon (`self.CurWeapon`))
  (bind (_bblockinghit _binitialoverlap _time _location) (`GameplayStatics.BreakHitResult` (`PlayerController.GetHitResultUnderCursorForObjects` (`GameplayStatics.GetPlayerController` 0) (`|MakeArray` "ObjectTypeQuery1" "ObjectTypeQuery2" "ObjectTypeQuery3" "ObjectTypeQuery4" "ObjectTypeQuery6" :!type "EObjectTypeQuery Enum") true)))
  (`Controller.SetControlRotation` (`GameplayStatics.GetPlayerController` 0) (`KismetMathLibrary.MakeRotator` 0.0 0.0 (.yaw (`KismetMathLibrary.FindLookAtRotation` (`self.K2_GetActorLocation`) _location))))
  (`self.K2_SetActorRotation` _curweapon (`KismetMathLibrary.FindLookAtRotation` (`self.K2_GetActorLocation` _curweapon) _location) false))

(fn `UserConstructionScript`)