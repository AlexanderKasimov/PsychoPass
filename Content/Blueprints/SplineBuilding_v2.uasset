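; SplineBuilding_v2 is a spline-driven building actor that, as wired, only sizes its list of building blocks.
; The Construction Script derives BlockCount from one block per whole 400 units of spline length.
; It then adds or removes BuildingBlockElements entries through a looped-back CompareInt until the array length matches.
; Nodes for spawning child actors at transforms along the spline are present but disconnected, and the event graph is empty.
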(fn `UserConstructionScript`
  (bind _buildingblockelements (`self.BuildingBlockElements`))
  (`|ExecutionSequence`
    (:`then_0`
      (set `self.BlockCount` (`.ReturnValue` (`KismetMathLibrary.FMod` (`SplineComponent.GetSplineLength` (`self.Spline`)) 400.0))))
    (:`then_1`
      (`/Engine/EditorBlueprintResources/StandardMacros.CompareInt` (`KismetArrayLibrary.Array_Length` (`self.BuildingBlockElements`)) (`self.BlockCount`) :!label _label
        (:`>`
          (`KismetArrayLibrary.Array_Remove` _buildingblockelements (`KismetArrayLibrary.Array_LastIndex` _buildingblockelements))
          (goto _label))
        (:`<`
          (`KismetArrayLibrary.Array_Add` (`self.BuildingBlockElements`))
          (goto _label))))))