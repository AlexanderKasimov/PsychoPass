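; SplineBuilding1 is a construction-script Blueprint that lays out child actors along a spline, apparently as repeating building pieces.
; It divides the spline length into whole 400-unit steps and adds a child actor component at each, oriented to the spline and unit-scaled.
; The components use manual attachment with transforms sampled in world space, and the event graph holds only disabled stubs.
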(fn `UserConstructionScript`
  (bind _spline (`self.Spline`))
  (for _index (range (`.ReturnValue` (`KismetMathLibrary.FMod` (`SplineComponent.GetSplineLength` (`self.Spline`)) 400.0)))
    (bind _returnvalue (* _index 400.0))
    (`AddComponent|NODE_AddChildActorComponent-0` :`bManualAttachment` true :`RelativeTransform` (`KismetMathLibrary.MakeTransform` (`SplineComponent.GetLocationAtDistanceAlongSpline` _spline _returnvalue "World") (`SplineComponent.GetRotationAtDistanceAlongSpline` _spline _returnvalue "World")))))