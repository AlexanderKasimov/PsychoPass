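; Sunken is an attacking actor with a skeletal mesh that damages the player through a sphere on a bone socket.
; The construction script creates AttackSphere and attaches it to the end-bone socket.
; From BeginPlay, a timeline blends CurTransform between Start and End, with a FlipFlop on finish to alternate reverse and forward playback.
; AttackSphere overlaps send a damage message to Player-tagged characters; look-at-player rotation is left unwired.
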(event `HitPlayer`
  (bind (_direction _newtrack_1) (`Timeline|Timeline_0`)
    (:`Update`
      (set `self.CurTransform` (`KismetMathLibrary.TLerp` (`SceneComponent.K2_GetComponentToWorld` (`self.Start`)) (`SceneComponent.K2_GetComponentToWorld` (`self.End`)) _newtrack_1)))
    (:`Finished`
      (`/Engine/EditorBlueprintResources/StandardMacros.FlipFlop`
        (:`A`
          (`TimelineComponent.ReverseFromEnd` (`self.Timeline_0`)))
        (:`B`
          (`TimelineComponent.PlayFromStart` (`self.Timeline_0`)))))))

(event `self.ReceiveTick`
  (params (DeltaSeconds :type "Float (single-precision)")))

(event `self.ReceiveBeginPlay`
  (`self.HitPlayer`))

(event `self.AttackSphere.OnComponentBeginOverlap`
  (params (OverlappedComponent :type "PrimitiveComponent Object Reference") (OtherActor :type "Actor Object Reference") (OtherComp :type "PrimitiveComponent Object Reference") (OtherBodyIndex :type Integer) (bFromSweep :type Boolean) (SweepResult :type "HitResult Structure (by ref)"))
  (bind _attacksphere (`self.AttackSphere`))
  (if (and (`KismetSystemLibrary.DoesImplementInterface` OtherActor "/Game/Blueprints/iCharacter.iCharacter_C") (`self.ActorHasTag` OtherActor "Player"))
    (message `/Game/Blueprints/iCharacter.ReceiveDamage` OtherActor "NewEnumerator0" (`GameplayStatics.MakeHitResult` false false 0.0 (`SceneComponent.K2_GetComponentLocation` _attacksphere) (0.0 0.0 0.0) (0.0 0.0 1.0) (0.0 0.0 1.0) null self _attacksphere))))

(fn `UserConstructionScript`
  (`|ExecutionSequence`
    (:`then_0`
      (bind _returnvalue (`AddComponent|NODE_AddSphereComponent-0` :`RelativeTransform` (`KismetMathLibrary.MakeTransform` (.location (`SceneComponent.GetSocketTransform` (`self.SkeletalMesh`) "Bone_005_endSocket" "RTS_Actor")) (.rotation (`SceneComponent.GetSocketTransform` (`self.SkeletalMesh`) "Bone_005_endSocket" "RTS_Actor")))))
      (bind _output_get (set `self.AttackSphere` _returnvalue))
      (`SceneComponent.K2_AttachToComponent` _output_get (`self.SkeletalMesh`) "Bone_005_endSocket" "SnapToTarget" "SnapToTarget" "KeepWorld" true))))