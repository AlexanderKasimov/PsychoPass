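; Enemy character Blueprint that reacts to projectile hits with dismemberment and ragdoll death.
; BeginPlay spawns the default controller and starts a timeline interpolating CurTransform between Start and End for hand movement.
; Projectile damage breaks the hit bone's constraint; hits outside arm or hand bones also enable mesh physics, disable capsule collision and set a lifespan.
; Construction stores a dynamic body material, but color randomization is disconnected and Hitted is an empty stub.
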(event `MoveHand`
  (bind (_direction _newtrack_1) (`Timeline|Timeline_0`)
    (:`Update`
      (set `self.CurTransform` (`KismetMathLibrary.TLerp` (`SceneComponent.K2_GetComponentToWorld` (`self.Start`)) (`SceneComponent.K2_GetComponentToWorld` (`self.End`)) _newtrack_1)))))

(event `self.ReceiveBeginPlay`
  (`self.SpawnDefaultController` self)
  (`self.MoveHand`))

(event `Hitted`)

(event `/Game/Blueprints/iCharacter.ReceiveDamage`
  (params (DamageType :type "/Game/Blueprints/Enum_DamageType Enum" :default "NewEnumerator0") (HitInfo :type "HitResult Structure"))
  (bind (_bblockinghit _binitialoverlap _time _location _impactpoint _normal _impactnormal _physmat _hitactor _hitcomponent _hitbonename) (`GameplayStatics.BreakHitResult` HitInfo))
  (bind _returnvalue (`KismetStringLibrary.Conv_NameToString` _hitbonename))
  (switch `/Game/Blueprints/Enum_DamageType` DamageType
    (:`NewEnumerator0`
      (`SkeletalMeshComponent.BreakConstraint` (`self.Mesh`) (* _impactnormal -80000.0) _impactpoint _hitbonename)
      (if (and (== (`KismetStringLibrary.FindSubstring` _returnvalue "arm") -1) (== (`KismetStringLibrary.FindSubstring` _returnvalue "hand") -1))
        (`self.SetLifeSpan` 15.0)
        (`PrimitiveComponent.SetSimulatePhysics` (`self.Mesh`) true)
        (`PrimitiveComponent.SetCollisionEnabled` (`self.CapsuleComponent`) "NoCollision")))))

(fn `RandomizeMaterial`)

(fn `UserConstructionScript`
  (bind _returnvalue (`PrimitiveComponent.CreateDynamicMaterialInstance` (`self.Mesh`) 0 null))
  (set `self.BodyMaterial` _returnvalue))