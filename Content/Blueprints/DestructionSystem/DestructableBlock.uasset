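; Destructible physics block that shatters into eight smaller blocks when its mesh takes a hit with a strong enough normal impulse.
; Eight arrow components mark the spawn transforms of the pieces, which spawn at half the arrows' scale and inherit the block's linear and angular velocity.
; Cut recursively spawns its own class while world X scale exceeds MaxCutLevel, otherwise it spawns UndestructableBlock pieces, and destroys the original either way.
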(event `self.StaticMesh.OnComponentHit`
  (params (HitComponent :type "PrimitiveComponent Object Reference") (OtherActor :type "Actor Object Reference") (OtherComp :type "PrimitiveComponent Object Reference") (NormalImpulse :type "Vector Structure") (Hit :type "HitResult Structure (by ref)"))
  (if (> (`KismetMathLibrary.VSize` NormalImpulse) 50000.0)
    (`self.Cut`)))

(fn `Cut`
  (locals (AngularVelocity :type "Vector Structure" :default (0.0 0.0 0.0)) (LinearVelocity :type "Vector Structure" :default (0.0 0.0 0.0)))
  (bind _staticmesh (`self.StaticMesh`))
  (bind _staticmesh_2 (`self.StaticMesh`))
  (if (> (.x (`SceneComponent.K2_GetComponentScale` (`self.StaticMesh`))) (`self.MaxCutLevel`))
    (bind _returnvalue (`PrimitiveComponent.GetPhysicsAngularVelocity` _staticmesh "None"))
    (set `local.AngularVelocity` _returnvalue)
    (bind _returnvalue_2 (`PrimitiveComponent.GetPhysicsLinearVelocity` _staticmesh "None"))
    (set `local.LinearVelocity` _returnvalue_2)
    (for _array_element (`self.Positions`)
      (bind _returnvalue_3 (`|SpawnActorFromClass` (`GameplayStatics.GetObjectClass` self) (`KismetMathLibrary.MakeTransform` (.location (`SceneComponent.K2_GetComponentToWorld` _array_element)) (.rotation (`SceneComponent.K2_GetComponentToWorld` _array_element)) (/ (.scale (`SceneComponent.K2_GetComponentToWorld` _array_element)) 2.0)) "Undefined" "OverrideRootScale" null null))
      (bind _staticmesh_3 (`/Game/Blueprints/DestructionSystem/DestructableBlock.StaticMesh` _returnvalue_3))
      (`PrimitiveComponent.SetPhysicsAngularVelocity` _staticmesh_3 (`local.AngularVelocity`) false "None")
      (`PrimitiveComponent.SetPhysicsLinearVelocity` _staticmesh_3 (`local.LinearVelocity`) false "None"))
    (`self.K2_DestroyActor`)
    (else
      (bind _returnvalue_4 (`PrimitiveComponent.GetPhysicsAngularVelocity` _staticmesh_2 "None"))
      (set `local.AngularVelocity` _returnvalue_4)
      (bind _returnvalue_5 (`PrimitiveComponent.GetPhysicsLinearVelocity` _staticmesh_2 "None"))
      (set `local.LinearVelocity` _returnvalue_5)
      (for _array_element_2 (`self.Positions`)
        (bind _returnvalue_6 (`|SpawnActorFromClass` "/Game/Blueprints/DestructionSystem/UndestructableBlock.UndestructableBlock_C" (`KismetMathLibrary.MakeTransform` (.location (`SceneComponent.K2_GetComponentToWorld` _array_element_2)) (.rotation (`SceneComponent.K2_GetComponentToWorld` _array_element_2)) (/ (.scale (`SceneComponent.K2_GetComponentToWorld` _array_element_2)) 2.0)) "Undefined" "OverrideRootScale" null null))
        (bind _staticmesh_4 (`/Game/Blueprints/DestructionSystem/UndestructableBlock.StaticMesh` _returnvalue_6))
        (`PrimitiveComponent.SetPhysicsAngularVelocity` _staticmesh_4 (`local.AngularVelocity`) false "None")
        (`PrimitiveComponent.SetPhysicsLinearVelocity` _staticmesh_4 (`local.LinearVelocity`) false "None"))
      (`self.K2_DestroyActor`))))

(fn `UserConstructionScript`
  (set `self.Positions` (`|MakeArray` (`self.Arrow`) (`self.Arrow1`) (`self.Arrow2`) (`self.Arrow3`) (`self.Arrow4`) (`self.Arrow5`) (`self.Arrow6`) (`self.Arrow7`))))