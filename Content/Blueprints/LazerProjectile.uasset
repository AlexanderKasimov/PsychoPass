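; Laser projectile that dismembers enemies and gets a random color when spawned.
; A mesh hit on an Enemy-tagged EnemyCharacter breaks the struck bone's constraint with an impulse along the impact normal.
; Unless the bone name contains "arm" or "hand", the enemy also ragdolls, loses capsule collision and is given a limited lifespan.
; The construction script creates the dynamic material that BeginPlay tints.
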(event `self.ReceiveBeginPlay`
  (`self.RandomizeMat`))

(event `self.Mesh.OnComponentHit`
  (params (HitComponent :type "PrimitiveComponent Object Reference") (OtherActor :type "Actor Object Reference") (OtherComp :type "PrimitiveComponent Object Reference") (NormalImpulse :type "Vector Structure") (Hit :type "HitResult Structure (by ref)"))
  (bind (_bblockinghit _binitialoverlap _time _location _impactpoint _normal _impactnormal _physmat _hitactor _hitcomponent _hitbonename) (`GameplayStatics.BreakHitResult` Hit))
  (bind _returnvalue (`KismetStringLibrary.Conv_NameToString` _hitbonename))
  ;[1 1 1] Dismember hited enemy
  (if (`self.ActorHasTag` OtherActor "Enemy")
    (bind _asenemy_character (cast `/Game/Blueprints/EnemyCharacter` OtherActor))
    (`SkeletalMeshComponent.BreakConstraint` (`Character.Mesh` _asenemy_character) (* _impactnormal 10000.0) _impactpoint _hitbonename)
    (if (and (== (`KismetStringLibrary.FindSubstring` _returnvalue "arm") -1) (== (`KismetStringLibrary.FindSubstring` _returnvalue "hand") -1))
      (`self.SetLifeSpan` _asenemy_character 15.0)
      (`PrimitiveComponent.SetSimulatePhysics` (`Character.Mesh` _asenemy_character) true)
      (`PrimitiveComponent.SetCollisionEnabled` (`Character.CapsuleComponent` _asenemy_character) "NoCollision"))))

(fn `RandomizeMat`
  (`MaterialInstanceDynamic.SetVectorParameterValue` (`self.LazerMat`) "Color" (make `LinearColor` (`KismetMathLibrary.RandomFloatInRange` 0.0 1.0) (`KismetMathLibrary.RandomFloatInRange` 0.0 1.0) (`KismetMathLibrary.RandomFloatInRange` 0.0 1.0))))

(fn `UserConstructionScript`
  (bind _returnvalue (`PrimitiveComponent.CreateDynamicMaterialInstance` (`self.Mesh`) 0 null))
  (set `self.LazerMat` _returnvalue))